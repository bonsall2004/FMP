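; BP_Berry is a collectible, edible berry item that restores a small random amount of health.
; When a third-person character overlaps its sphere, it adds one of its data-component item ID to that character's inventory and destroys itself.
; UseItem prints a debug "Hello", adds the random health to the using character and plays an eating montage.
; LookAt returns an empty string.
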(event OnComponentBeginOverlap(Sphere)
  (params (OverlappedComponent :type Primitive%20Component%20Object%20Reference) (OtherActor :type Actor%20Object%20Reference) (OtherComp :type Primitive%20Component%20Object%20Reference) (OtherBodyIndex :type Integer) (bFromSweep :type Boolean) (SweepResult :type Hit%20Result%20Structure%20%28by%20ref%29))
  (bind _asbp_third_person_character (Utilities|Casting|CastToBP_ThirdPersonCharacter OtherActor))
  (Utilities|IsValid (Variables|/Game/ThirdPerson/Blueprints/BP_ThirdPersonCharacter.BP_ThirdPersonCharacter_C|GetInventoryComponent _asbp_third_person_character)
    (:Is%20Valid
      (Default|AddItem (Variables|/Game/ThirdPerson/Blueprints/BP_ThirdPersonCharacter.BP_ThirdPersonCharacter_C|GetInventoryComponent _asbp_third_person_character) (.RowName (Utilities|Struct|BreakDataTableRowHandle (Variables|/Game/BON21001291/Inventory/Components/ItemDataComponent.ItemDataComponent_C|GetItemID (Variables|Default|GetItemDataComponent)))) 1)
      (Actor|DestroyActor))))

(event EventBeginPlay)

(event Collision|EventActorBeginOverlap
  (params (OtherActor :type Actor%20Object%20Reference)))

(event EventTick
  (params (DeltaSeconds :type Float%20%28single-precision%29)))

(event EventUseItem
  (params (Character%20Ref :type Actor%20Object%20Reference))
  (bind _asbp_third_person_character (Utilities|Casting|CastToBP_ThirdPersonCharacter Character%20Ref))
  (Development|PrintString "Hello")
  (Default|AddHealth _asbp_third_person_character (Math|Conversions|ToFloat(Integer) (Math|Random|RandomInteger 20)))
  (Animation|PlayAnimMontage _asbp_third_person_character "/Game/BON21001291/Character/Animations/Montages/AnimM_Eat.AnimM_Eat" 1.0 "None"))

(fn ConstructionScript
  (|CallParentFunction))

(fn Lookat
  (return ""))