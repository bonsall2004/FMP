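; BP_Strawberry is a pickup item Blueprint for a strawberry perk, driven by an item data table.
; The construction script looks up the ItemDataComponent's row and sets the static mesh from it, so the placed actor shows the correct model.
; LookAt reads the same row and returns a "Pick Up {Item}" prompt using the item's name.
; The event graph holds no active logic.
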(event EventBeginPlay)

(event Collision|EventActorBeginOverlap
  (params (OtherActor :type Actor%20Object%20Reference)))

(event EventTick
  (params (DeltaSeconds :type Float%20%28single-precision%29)))

(fn ConstructionScript
  (bind _itemdatacomponent (Variables|Default|GetItemDataComponent))
  (bind _itemid (Variables|/Game/BON21001291/Inventory/Components/ItemDataComponent.ItemDataComponent_C|GetItemID _itemdatacomponent))
  (bind _returnvalue (Utilities|GetDataTableRow (.datatable _itemid) (.rowname _itemid))
    (:then
      (Components|StaticMesh|SetStaticMesh (Variables|Default|GetMesh) (.Mesh (Utilities|Struct|BreakItemStructure _returnvalue))))))

(fn Lookat
  (bind _itemdatacomponent (Variables|Default|GetItemDataComponent))
  (bind _itemid (Variables|/Game/BON21001291/Inventory/Components/ItemDataComponent.ItemDataComponent_C|GetItemID _itemdatacomponent))
  (bind _returnvalue (Utilities|GetDataTableRow (.datatable _itemid) (.rowname _itemid))
    (:then
      (return (Utilities|Text|FormatText "Pick Up {Item}" (.ItemName (Utilities|Struct|BreakItemStructure _returnvalue)))))))